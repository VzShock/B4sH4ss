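; B_Door is a level-mechanic door Blueprint that opens when enough pressure switches are active.
; SwitchActivate and SwitchDeactivate raise or lower an active-switch count and compare it with the required number.
; Reaching that number plays the OpenClose timeline and falling short reverses it, with its DoorPosition track driving the Door's relative Z location.
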(event `SwitchActivate`
  ;[1 1 1] Check if we got the right switch
  (`/Engine/EditorBlueprintResources/StandardMacros.IncrementInt` (`self.PressureSwitchesActive`)
    (:`  `
      (if (>= (`self.PressureSwitchesActive`) (`self.PressureSwitchesNeeded`))
        (bind (_direction _doorposition) (`Timeline|OpenClose` :!label _label)
          (:`Update`
            (`SceneComponent.K2_SetRelativeLocation` (`self.Door`) (`KismetMathLibrary.MakeVector` 0.0 0.0 _doorposition) false false)))
        (else
          (goto _label :!via `Reverse`))))))

(event `SwitchDeactivate`
  ;[1 1 1] Do we have enough switches to open the door ?
  (`/Engine/EditorBlueprintResources/StandardMacros.DecrementInt` (`self.PressureSwitchesActive`)
    (:`  `
      (if (>= (`self.PressureSwitchesActive`) (`self.PressureSwitchesNeeded`))
        (goto _label)
        (else
          (goto _label :!via `Reverse`))))))

(fn `UserConstructionScript`)