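; Tutorial text trigger actor that shows a configurable text while the third-person player character is inside its overlap area.
; BeginPlay fills the TextRender component from TextInput.
; On overlap it moves the text to the character's location plus TextOffset, rotates it to face the character and makes it visible.
; The text stays where placed, without following the character, and hides when the overlap ends.
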(event `self.ReceiveBeginPlay`
  ;[0.1386 1 0.3117] Load text
  (`TextRenderComponent.K2_SetText` (`self.TextRender`) (`self.TextInput`)))

(event `self.ReceiveActorBeginOverlap`
  (params (OtherActor :type "Actor Object Reference"))
  ;[0.4168 0.4665 1] Load text by offset and rotation
  (bind _asbp_third_person_character (cast `/Game/ThirdPerson/Blueprints/BP_ThirdPersonCharacter` OtherActor))
  ;;[1 0.7408 0.2336] Set location by offset
  (`SceneComponent.K2_SetWorldLocation` (`self.TextRender`) (+ (`self.K2_GetActorLocation` _asbp_third_person_character) (`self.TextOffset`)) false false)
  ;;[1 0.1781 0.1781] find and set good rotation
  (`SceneComponent.K2_SetWorldRotation` (`self.TextRender`) (`KismetMathLibrary.FindLookAtRotation` (`SceneComponent.K2_GetComponentLocation` (`self.TextRender`)) (`self.K2_GetActorLocation` _asbp_third_person_character)) false false)
  (`SceneComponent.SetVisibility` (`self.TextRender`) true false))

(event `self.ReceiveActorEndOverlap`
  (params (OtherActor :type "Actor Object Reference"))
  ;[1 1 1] Remove text on screen
  (cast `/Game/ThirdPerson/Blueprints/BP_ThirdPersonCharacter` OtherActor)
  (`SceneComponent.SetVisibility` (`self.TextRender`) false false))

(fn `UserConstructionScript`)