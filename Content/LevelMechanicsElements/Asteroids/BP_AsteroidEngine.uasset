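; Asteroid ring actor that procedurally builds a belt of instanced meshes and slowly spins it around its local Z axis on Tick.
; The construction script sets the HISM mesh and cull distances, then adds instances over a length-by-width grid, scaled by width index.
; AsteroidTransformation wraps that grid into a ring, using a random stream to jitter positions and blend ring-aligned rotations toward random ones.
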(event `self.ReceiveTick`
  (params (DeltaSeconds :type "Float (single-precision)"))
  (`self.K2_AddActorLocalRotation` (`KismetMathLibrary.RotatorFromAxisAndAngle` (0.0 0.0 1.0) (* DeltaSeconds (`self.RotationSpeed`)))))

(fn `AsteroidTransformation`
  (params (`Index from width loop` :type Integer) (`NB of instances by width` :type Integer) (`Idx from Length loop` :type Integer) (`NB of instances by length` :type Integer))
  (returns (OutLocation :type "Vector Structure") (OutRotating :type "Rotator Structure"))
  (bind _returnvalue (`KismetMathLibrary.MakeVector` 0.0 0.0 1.0))
  (bind _transformrand (`self.TransformRand`))
  (bind _returnvalue_2 (`KismetMathLibrary.RotateAngleAxis` (+ (+ (* (- (`KismetMathLibrary.RandomFloatFromStream` _transformrand) 0.5) (`self.RandZAxisPos`) (`self.RingWitdh`)) (* (`KismetMathLibrary.RandomUnitVectorFromStream` _transformrand) (`self.RandPosition`))) (`KismetMathLibrary.MakeVector` 0.0 (+ (`self.RingRadius`) (* (- (/ (`KismetMathLibrary.Conv_IntToDouble` `Index from width loop`) (`KismetMathLibrary.Conv_IntToDouble` `NB of instances by width`)) 0.5) (`self.RingWitdh`))))) (* (/ (`KismetMathLibrary.Conv_IntToDouble` `Idx from Length loop`) (`KismetMathLibrary.Conv_IntToDouble` `NB of instances by length`)) 360.0) _returnvalue))
  (return _returnvalue_2 (`KismetMathLibrary.RLerp` (`KismetMathLibrary.MakeRotFromYZ` (`KismetMathLibrary.Cross_VectorVector` _returnvalue _returnvalue_2) _returnvalue) (`KismetMathLibrary.RandomRotatorFromStream` (`self.TransformRand`) true) (`self.RandRotation`) true)))

(fn `UserConstructionScript`
  (bind _hierarchicalinstancedstaticspawn_ (`self.HierarchicalInstancedStaticSpawn*`))
  (bind _instancecountbylength (`self.InstanceCountByLength`))
  (bind _instancecountbywitdh (`self.InstanceCountByWitdh`))
  (`|ExecutionSequence`
    (:`then_0`
      (`StaticMeshComponent.SetStaticMesh` _hierarchicalinstancedstaticspawn_ (`self.InstanceMesh`)))
    (:`then_1`
      (`InstancedStaticMeshComponent.SetCullDistances` _hierarchicalinstancedstaticspawn_ (`self.CullingNear`) (`self.CullingFar`)))
    (:`then_2`
      (for _index (range _instancecountbylength)
        (for _index_2 (range _instancecountbywitdh)
          (bind (_outlocation _outrotating) (`self.AsteroidTransformation` _index_2 _instancecountbywitdh _index _instancecountbylength))
          (`InstancedStaticMeshComponent.AddInstance` (`self.HierarchicalInstancedStaticSpawn*`) (`KismetMathLibrary.MakeTransform` _outlocation _outrotating (`KismetMathLibrary.Conv_DoubleToVector` (* _index_2 (`self.RandScaleMinimum`)))) false))))))